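; BP_Moon is a moon actor that orbits the BP_Planet actor in a circle on the XY plane.
; Each Tick calls UpdateLocation, then advances Angle by a fixed, frame-rate-dependent step, printing it and resetting it once past a full turn.
; UpdateLocation looks up the planet with GetActorOfClass on every call and offsets the moon's root from the planet's position using Radio and the cosine and sine of Angle.
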(event EventBeginPlay
  (|CallParentFunction) ; This node is disabled and will not be called.\nDrag off pins to build functionality.
)

(event Collision|EventActorBeginOverlap
  (params (OtherActor :type Actor%20Object%20Reference)))

(event EventTick
  (params (DeltaSeconds :type Float%20%28single-precision%29))
  (|CallParentFunction DeltaSeconds)
  (CallFunction|UpdateLocation (Variables|Default|GetRadio) (Variables|Default|GetAngle))
  (if (<= (Variables|Default|GetAngle) 3.6e+02)
    (Variables|Default|SetAngle (+ (Variables|Default|GetAngle) 0.2))
    (Development|PrintString (Utilities|String|ToString(Float) (Variables|Default|GetAngle)))
    (else
      (Variables|Default|SetAngle 0.0))))

(fn ConstructionScript
  (|CallParentFunction))

(fn UpdateLocation
  (params (Radio :type Float%20%28double-precision%29) (Angle :type Float%20%28double-precision%29))
  (Variables|Default|SetRadio Radio)
  (Variables|Default|SetAngle Angle)
  (bind _returnvalue (Actor|GetActorOfClass "/Game/Blueprints/BP_Planet.BP_Planet_C"))
  (Utilities|IsValid _returnvalue
    (:Is%20Valid
      (LocalVariables|SetBP_Planet _returnvalue)
      (Transformation|SetWorldLocation (Variables|Default|GetDefaultSceneRoot) (Math|Vector|MakeVector (+ (.x (Transformation|GetWorldLocation (Variables|/Script/Engine.Actor|GetRootComponent (LocalVariables|GetBP_Planet)))) (* (Variables|Default|GetRadio) (Math|Trig|Cos(Degrees) (Variables|Default|GetAngle)))) (+ (.y (Transformation|GetWorldLocation (Variables|/Script/Engine.Actor|GetRootComponent (LocalVariables|GetBP_Planet)))) (* (Variables|Default|GetRadio) (Math|Trig|Sin(Degrees) (Variables|Default|GetAngle)))) 0.0) false false))))