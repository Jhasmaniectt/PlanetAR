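; BP_Planet is a planet actor that spins around its yaw axis each Tick at a speed set through RotatePlanet.
; SetPlanetMesh looks up the named row in DT_SM_Planets to apply mesh and scale, then toggles the optional complement: Saturn's ring or a cloud layer for other planets.
; SetInitialLocation moves it to its stored InitialLocation, and BeginPlay enables player input.
; Debug prints and a CallMeshTouched call remain unwired.
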(event EventTick
  (params (DeltaSeconds :type Float%20%28single-precision%29))
  (Transformation|AddLocalRotation (Variables|Default|GetSM_Planet) (Math|Rotator|MakeRotator 0.0 0.0 (* DeltaSeconds (Variables|Default|GetVel_Rotation))) false false))

(event EventBeginPlay
  (Variables|Default|SetPlanetSMs "/Game/Blueprints/DT_SM_Planets.DT_SM_Planets")
  (Input|EnableInput (Game|GetPlayerController 0)))

(fn ConstructionScript)

(fn SetInitialLocation
  (Transformation|SetActorLocation (Variables|Default|GetInitialLocation) false false))

(fn RotatePlanet
  (params (Velocity :type Float%20%28double-precision%29))
  (Variables|Default|SetVel_Rotation Velocity))

(fn SetPlanetMesh
  (params (Name%20Planet :type Name) (Complement :type Boolean))
  (bind _output_get (Variables|Default|SetPlanet Name%20Planet))
  (bind _returnvalue (Utilities|GetDataTableRow "/Game/Blueprints/DT_SM_Planets.DT_SM_Planets" _output_get)
    (:then
      (Components|StaticMesh|SetStaticMesh (Variables|Default|GetSM_Planet) (.mesh _returnvalue))
      (Transformation|SetWorldScale3D (Variables|Default|GetSM_Planet) (Math|Vector|MakeVector (.scale _returnvalue) (.scale _returnvalue) (.scale _returnvalue)))
      (if Complement
        (if (== (Variables|Default|GetPlanet) "Saturn_SM")
          (Development|SetHiddeninGame (Variables|Default|GetCloud) true false)
          (Development|SetHiddeninGame (Variables|Default|GetSat_Ring) false false)
          (else
            (Development|SetHiddeninGame (Variables|Default|GetSat_Ring) true false)
            (Development|SetHiddeninGame (Variables|Default|GetCloud) false false)))
        (else
          (Development|SetHiddeninGame (Variables|Default|GetCloud) true false))))))