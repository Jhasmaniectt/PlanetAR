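; BP_Monn2 is a moon actor that spins on its own axis and circles the BP_Planet in the level.
; Tick yaws the mesh by VelRotation, which RotatePlanet sets, and advances the orbit angle by VelTraslacion scaled down by 27.
; UpdateMoonLocation looks up the planet every frame and uses cosine and sine to place the moon around its X/Y position.
; BeginPlay stores the planet mesh table and enables input, but SetPlanetMesh is empty.
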(event EventTick
  (params (DeltaSeconds :type Float%20%28single-precision%29))
  (Transformation|AddLocalRotation (Variables|Default|GetSM_Planet) (Math|Rotator|MakeRotator 0.0 0.0 (* DeltaSeconds (Variables|Default|GetVel_Rotation))) false false)
  (CallFunction|UpdateMoonLocation (Variables|Default|GetRadius) (Variables|Default|GetAngle))
  (if (<= (Variables|Default|GetAngle) 3.6e+02)
    (Variables|Default|SetAngle (+ (Variables|Default|GetAngle) (/ (* DeltaSeconds (Variables|Default|GetVel_Traslacion)) 27.0)))
    (else
      (Variables|Default|SetAngle 0.0))))

(event EventBeginPlay
  (Variables|Default|SetPlanetSMs "/Game/Blueprints/DT_SM_Planets.DT_SM_Planets")
  (Input|EnableInput (Game|GetPlayerController 0)))

(fn ConstructionScript)

(fn RotatePlanet
  (params (Velocity :type Float%20%28double-precision%29))
  (Variables|Default|SetVel_Rotation Velocity))

(fn SetPlanetMesh
  (params (Name%20Planet :type Name) (Complement :type Boolean)))

(fn UpdateMoonLocation
  (params (Radius :type Float%20%28double-precision%29) (Angle :type Float%20%28double-precision%29))
  (bind _returnvalue (Actor|GetActorOfClass "/Game/Blueprints/BP_Planet.BP_Planet_C"))
  (Utilities|IsValid _returnvalue
    (:Is%20Valid
      (Variables|Default|SetBP_Planet _returnvalue)
      (Transformation|SetWorldLocation (Variables|Default|GetDefaultSceneRoot) (Math|Vector|MakeVector (+ (.x (Transformation|GetWorldLocation (Variables|/Script/Engine.Actor|GetRootComponent (Variables|Default|GetBP_Planet)))) (* (Variables|Default|GetRadius) (Math|Trig|Cos(Degrees) (Variables|Default|GetAngle)))) (+ (.y (Transformation|GetWorldLocation (Variables|/Script/Engine.Actor|GetRootComponent (Variables|Default|GetBP_Planet)))) (* (Variables|Default|GetRadius) (Math|Trig|Sin(Degrees) (Variables|Default|GetAngle)))) 0.0) false false))))